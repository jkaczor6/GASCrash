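; Player primary attack ability for the GASCrash project that plays a melee swing and damages whatever it hits.
; A FlipFlop alternates between two attack montages, ending the ability when either finishes, blends out or is stopped.
; In parallel it waits for the primary gameplay event tag, then runs a hit box overlap test, sends hit reacts and applies GE_PlayerDamage at the ability's level to each actor found.
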(event `self.K2_ActivateAbility`
  (bind _returnvalue (`self.GetAbilitySystemComponentFromActorInfo`))
  (`|ExecutionSequence`
    (:`then_0`
      ;[0.913 0 0 0.5] Play Attack Montage
      (`/Engine/EditorBlueprintResources/StandardMacros.FlipFlop`
        (:`A`
          (`AbilityTask_PlayMontageAndWait.CreatePlayMontageAndWaitProxy` "None" "/Game/GASCrash/Characters/PlayerCharacter/Animations/GC_Primary_A_Montage.GC_Primary_A_Montage"
            (:`OnCompleted`
              _)
            (:`OnBlendOut`
              _)
            (:`OnInterrupted`
              _)
            (:`OnCancelled`
              _))
          (`self.K2_EndAbility`))
        (:`B`
          (`AbilityTask_PlayMontageAndWait.CreatePlayMontageAndWaitProxy` "None" "/Game/GASCrash/Characters/PlayerCharacter/Animations/GC_Primary_B_Montage.GC_Primary_B_Montage"
            (:`OnCompleted`
              _)
            (:`OnBlendOut`
              _)
            (:`OnInterrupted`
              _)
            (:`OnCancelled`
              _))
          (`self.K2_EndAbility`))))
    (:`then_1`
      (`AbilityTask_WaitGameplayEvent.WaitGameplayEvent` (struct :`TagName` "GCTags.Events.Player.Primary") null
        (:`EventReceived`
          (bind _returnvalue_2 (`self.HitBoxOverlapTest`))
          (`self.SendHitReactEventToActors` _returnvalue_2)
          (for _array_element _returnvalue_2
            (`AbilitySystemComponent.BP_ApplyGameplayEffectSpecToTarget` _returnvalue (`AbilitySystemComponent.MakeOutgoingSpec` :`self` _returnvalue :`GameplayEffectClass` "/Game/GASCrash/AbilitySystem/GameplayEffects/Player/GE_PlayerDamage.GE_PlayerDamage_C" :`Level` (`KismetMathLibrary.Conv_IntToDouble` (`self.GetAbilityLevel`))) (`AbilitySystemBlueprintLibrary.GetAbilitySystemComponent` _array_element))))))))

(event `self.K2_OnEndAbility`
  (params (bWasCancelled :type Boolean))
  (if (`self.bDrawDebugs`)
    (`KismetSystemLibrary.PrintString` "GA_Primary: Ended")))