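; Player gameplay ability that turns hit-react and death gameplay events into impact gameplay cues.
; On activation it starts two parallel WaitGameplayEvent listeners and never explicitly ends.
; Hit-react events execute the HitReact cue, passing on the payload's effect context, instigator and source object.
; Death events activate the Death ability by tag, then execute the BurstImpact cue on the avatar with the same payload data.
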(event `self.K2_ActivateAbility`
  (`|ExecutionSequence`
    (:`then_0`
      (bind (_asynctaskproxy _payload) (`AbilityTask_WaitGameplayEvent.WaitGameplayEvent` (struct :`TagName` "GCTags.Events.Player.HitReact") null)
        (:`EventReceived`
          (bind (_eventtag _instigator _target _optionalobject _optionalobject2 _contexthandle) (break `GameplayEventData` _payload))
          (`self.K2_ExecuteGameplayCueWithParams` (struct :`TagName` "GameplayCue.HitReact") (`AbilitySystemBlueprintLibrary.MakeGameplayCueParameters` 0.0 0.0 _contexthandle (struct) (struct) (struct) (struct) (0.0 0.0 0.0) (0.0 0.0 0.0) _instigator null _optionalobject)))))
    (:`then_1`
      (bind (_asynctaskproxy_2 _payload_2) (`AbilityTask_WaitGameplayEvent.WaitGameplayEvent` (struct :`TagName` "GCTags.Events.Player.Death") null)
        (:`EventReceived`
          (`AbilitySystemComponent.TryActivateAbilitiesByTag` (`self.GetAbilitySystemComponentFromActorInfo`) (`BlueprintGameplayTagLibrary.MakeGameplayTagContainerFromTag` (`BlueprintGameplayTagLibrary.MakeLiteralGameplayTag` (struct :`TagName` "GCTags.GCAbilities.Death"))) true)
          (bind (_eventtag_2 _instigator_2 _target_2 _optionalobject_2 _optionalobject2_2 _contexthandle_2) (break `GameplayEventData` _payload_2))
          (`GameplayCueFunctionLibrary.ExecuteGameplayCueOnActor` (`self.GetAvatarActorFromActorInfo`) (struct :`TagName` "GameplayCue.BurstImpact") (`AbilitySystemBlueprintLibrary.MakeGameplayCueParameters` 0.0 0.0 _contexthandle_2 (struct) (struct) (struct) (struct) (0.0 0.0 0.0) (0.0 0.0 0.0) _instigator_2 null _optionalobject_2)))))))