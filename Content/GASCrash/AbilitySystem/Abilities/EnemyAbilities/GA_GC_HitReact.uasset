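; Enemy Gameplay Ability that plays a directional hit reaction.
; On activation it waits for the Enemy.HitReact gameplay event, then caches direction vectors relative to the event's Instigator.
; The avatar's forward and the vector to the instigator resolve to a hit direction name, used to jump to the matching section of a single hit react montage.
; The ability never calls EndAbility in this graph, and debug prints are gated by DrawDebugs.
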(event `self.K2_ActivateAbility`
  (bind (_asynctaskproxy _payload) (`AbilityTask_WaitGameplayEvent.WaitGameplayEvent` (struct :`TagName` "GCTags.Events.Enemy.HitReact") null)
    (:`EventReceived`
      (`self.PrintDebugEventReceived` _payload)
      (`self.CacheHitDirectionVectors` (`.Instigator` (break `GameplayEventData` _payload)))
      (`|ExecutionSequence`
        (:`then_0`
          ;[0.913 0 0 0.5] Cache Hit Direction Name
          (set `self.HitDirectionName` (`GC_BlueprintLibrary.GetHitDirectionName` (`GC_BlueprintLibrary.GetHitDirection` (`self.AvatarForward`) (`self.ToInstigator`))))
          ;[0 0.02136 0.15 0.5] Debug for Hit Direction
          (`self.bDrawDebugs`
            (:`then`
              (`KismetSystemLibrary.PrintString` (`KismetStringLibrary.Conv_NameToString` (`self.HitDirectionName`))))
            (:`else`)))
        (:`then_1`
          ;[0.913 0 0 0.5] Play Montage And Jump to the correct Hit React Montage Section
          (`AbilityTask_PlayMontageAndWait.CreatePlayMontageAndWaitProxy` "None" (`self.HitReactMontage`)
            (:`then`
              (`self.MontageJumpToSection` (`self.HitDirectionName`)))))))))

(fn `PrintDebugEventReceived`
  (params (GameplayEventData :type "GameplayEventData Structure (by ref)"))
  (`self.bDrawDebugs`
    (:`then`
      (`KismetSystemLibrary.PrintString` (`KismetStringLibrary.Concat_StrStr` "GA_GC_HitReact: Received Event from: " (`KismetSystemLibrary.GetDisplayName` (`.Instigator` (break `GameplayEventData` GameplayEventData)))) true true (struct :`R` 0.404313 :`B` 0.645833 :`A` 1.0)))
    (:`else`)))