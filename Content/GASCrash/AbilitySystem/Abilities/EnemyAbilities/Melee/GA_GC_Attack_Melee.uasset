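; Enemy melee attack Gameplay Ability that plays a random attack montage and damages the player when the swing connects.
; A Dead-tagged owner skips the attack and only sends the EndAttack event.
; Alongside the montage, a one-shot wait for the MeleeTraceHit event applies set-by-caller melee damage with impact particles.
; The ability ends when the montage finishes, is interrupted or is cancelled, sending EndAttack to the avatar.
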(event `self.K2_ActivateAbility`
  (if (`GameplayTagAssetInterface.HasMatchingGameplayTag` (`self.GetAbilitySystemComponentFromActorInfo`) (struct :`TagName` "GCTags.Status.Dead"))
    (`AbilitySystemBlueprintLibrary.SendGameplayEventToActor` (`self.GetAvatarActorFromActorInfo`) (struct :`TagName` "GCTags.Events.Enemy.EndAttack"))
    (else
      (`|ExecutionSequence`
        (:`then_0`
          (`AbilityTask_PlayMontageAndWait.CreatePlayMontageAndWaitProxy` "None" (`KismetArrayLibrary.Array_Random` (`self.AttackMontages`))
            (:`OnCompleted`
              _)
            (:`OnInterrupted`
              _)
            (:`OnCancelled`
              _))
          (`self.K2_EndAbility`))
        (:`then_1`
          (bind (_asynctaskproxy _payload) (`AbilityTask_WaitGameplayEvent.WaitGameplayEvent` (struct :`TagName` "GCTags.Events.Enemy.MeleeTraceHit") null true)
            (:`EventReceived`
              (`GC_BlueprintLibrary.SendDamageEventToPlayer` (`.Target` (break `GameplayEventData` _payload)) (`self.Damage Effect`) _payload (`BlueprintGameplayTagLibrary.MakeLiteralGameplayTag` (struct :`TagName` "GCTags.SetByCaller.Melee")) 10.0 (`BlueprintGameplayTagLibrary.MakeLiteralGameplayTag` (struct :`TagName` "GCTags.None")) (`self.ImpactParticles`)))))))))

(event `self.K2_OnEndAbility`
  (params (bWasCancelled :type Boolean))
  (`AbilitySystemBlueprintLibrary.SendGameplayEventToActor` (`self.GetAvatarActorFromActorInfo`) (struct :`TagName` "GCTags.Events.Enemy.EndAttack")))