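; Gameplay ability that handles a GC character's death and in-place revival.
; On activation it starts the death montage and applies GE_Death to the owner.
; When the montage completes, is interrupted or is cancelled, RespawnCharacter removes effects granting the Status.Dead tag, resets the GC_BaseCharacter's attributes on authority only, and ends the ability.
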(event `self.K2_ActivateAbility`
  (bind _returnvalue (`self.GetAbilitySystemComponentFromActorInfo`))
  (`AbilityTask_PlayMontageAndWait.CreatePlayMontageAndWaitProxy` "None" (`self.DeathMontage`)
    (:`then`
      (`AbilitySystemComponent.BP_ApplyGameplayEffectSpecToSelf` _returnvalue (`AbilitySystemComponent.MakeOutgoingSpec` :`self` _returnvalue :`GameplayEffectClass` "/Game/GASCrash/AbilitySystem/GameplayEffects/GE_Death.GE_Death_C" :`Level` 1.0)))
    (:`OnCompleted`
      (`self.RespawnCharacter` :!label _label))
    (:`OnInterrupted`
      (goto _label))
    (:`OnCancelled`
      (goto _label))))

(event `RespawnCharacter`
  (`|ExecutionSequence`
    (:`then_0`
      (`self.BP_RemoveGameplayEffectFromOwnerWithGrantedTags` (struct :`GameplayTags` (struct :`(TagName` "GCTags.Status.Dead"))) 1))
    (:`then_1`
      (`self.K2_HasAuthority`
        (:`True`
          (bind _asgc_base_character (cast `GC_BaseCharacter` (`self.GetAvatarActorFromActorInfo`)))
          (`GC_BaseCharacter.ResetAttributes` _asgc_base_character))))
    (:`then_2`
      (`self.K2_EndAbility`))))